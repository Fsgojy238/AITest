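; BP_Player is the player Blueprint, wired with debug-style key bindings that drive enemy AI state and senses.
; Key 1 finds a BP_Enemy_Base, casts its controller to AIC_Enemy_Base, and flip-flops it between attacking the player and passive.
; X emits a noise at the player's location, while F reports a damage event on the found enemy to trigger AI perception.
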(event `Key|One`
  (params (Key :type "Key Structure"))
  (:`Pressed`
    (bind _returnvalue (`GameplayStatics.GetActorOfClass` "/Game/Enemy/BP_Enemy_Base.BP_Enemy_Base_C"))
    (bind _asaic_enemy_base (cast `/Game/Enemy/AIC_Enemy_Base` (`AIBlueprintHelperLibrary.GetAIController` _returnvalue)))
    (`/Engine/EditorBlueprintResources/StandardMacros.FlipFlop`
      (:`A`
        (`/Game/Enemy/AIC_Enemy_Base.SetStateAsAttacking` _asaic_enemy_base self))
      (:`B`
        (`/Game/Enemy/AIC_Enemy_Base.SetStateAsPassive` _asaic_enemy_base)))))

(event `Key|X`
  (params (Key :type "Key Structure"))
  (:`Pressed`
    (`self.MakeNoise` 1.0 self (`self.K2_GetActorLocation`))))

(event `Key|F`
  (params (Key :type "Key Structure"))
  (:`Pressed`
    (bind _returnvalue (`GameplayStatics.GetActorOfClass` "/Game/Enemy/BP_Enemy_Base.BP_Enemy_Base_C"))
    (`AISense_Damage.ReportDamageEvent` _returnvalue self 10.0 (`self.K2_GetActorLocation`))))

(fn `UserConstructionScript`
  (`parent.UserConstructionScript`))