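; BP_PatrolRoute is a spline-based patrol route for enemy AI that exposes one waypoint at a time.
; GetSplinePointWorldLocation returns the world location of the spline point at the current PatrolRouteIndex.
; IncrementPatrolRoute steps the index by Direction, ping-ponging along the route by reversing when it equals the point count (one past the last point) or zero.
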(event `IncrementPatrolRoute`
  (set `self.PatrolRouteIndex` (+ (`self.PatrolRouteIndex`) (`self.Direction`)))
  (if (== (`self.PatrolRouteIndex`) (`SplineComponent.GetNumberOfSplinePoints` (`self.Spline`)))
    (set `self.Direction` -1)
    (elif (== (`self.PatrolRouteIndex`) 0)
      (set `self.Direction` 1))))

(fn `GetSplinePointWorldLocation`
  (returns (WorldLocation :type "Vector Structure"))
  (return (`SplineComponent.GetLocationAtSplinePoint` (`self.Spline`) (`self.PatrolRouteIndex`) "World")))

(fn `UserConstructionScript`)