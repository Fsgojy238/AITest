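; BP_Enemy_Range is a rifle-wielding ranged enemy that extends a parent enemy class.
; On BeginPlay it spawns a rifle and attaches it to the mesh's hand socket.
; Attack plays a fire montage whose notify traces from weapon to AI target, applying hitscan damage if nothing blocks, and completion signals attack end.
; It also defines walk speeds per locomotion state and its ideal attack and strafe range.
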(event `self.ReceiveBeginPlay`
  (`parent.ReceiveBeginPlay`)
  (`self.EquipWeapon`))

(event `/Game/Enemy/BPI_Enemy.EquipWeapon`
  (bind _returnvalue (`|SpawnActorFromClass` "/Game/Weapons/BP/BP_Weapon_Rifle.BP_Weapon_Rifle_C" (`self.GetTransform`) "Undefined" "MultiplyWithRoot" null null))
  (bind _output_get (set `self.WeaponActor` _returnvalue))
  (`self.K2_AttachToComponent` _output_get (`self.Mesh`) "RifleSocket" "SnapToTarget" "SnapToTarget" "SnapToTarget" true)
  (set `self.bIsWieldingWeapon` true))

(event `/Game/Enemy/BPI_Enemy.Attack`
  (bind _notifyname (`|PlayMontage` (`self.Mesh`) "/Game/Enemy/Enemy_Range/Anim/Montages/rifle-fire_Montage.rifle-fire_Montage")
    (:`OnCompleted`
      (`self.OnAttackEnd`))
    (:`OnNotifyBegin`
      (switch `name` _notifyname
        (:`Fire`
          (bind _asaic_enemy_base (cast `/Game/Enemy/AIC_Enemy_Base` (`AIBlueprintHelperLibrary.GetAIController` self)))
          (bind _attacktarget (`/Game/Enemy/AIC_Enemy_Base.AttackTarget` _asaic_enemy_base))
          (bind (_outhit _returnvalue) (`KismetSystemLibrary.LineTraceSingle` :`Start` (`self.K2_GetActorLocation` (`self.WeaponActor`)) :`End` (`self.K2_GetActorLocation` _attacktarget) :`TraceChannel` "TraceTypeQuery1" :`DrawDebugType` "Persistent"))
          (if (not _returnvalue)
            (message `/Game/DamageSystem/BPI_Damagable.TakeDamage` _attacktarget (make `/Game/DamageSystem/S_DamageInfo` 5.0 "NewEnumerator2" "NewEnumerator1") null)))))))

(fn `GetIdealRange`
  (returns (AttackRadius :type "Float (double-precision)") (StrafeRadius :type "Float (double-precision)"))
  (return 600.0 600.0))

(fn `SetMovementSpeed`
  (params (InLocomotionState :type "/Game/Enemy/Enum/E_LocomotionState Enum" :default "NewEnumerator0"))
  (returns (Speed :type "Float (double-precision)"))
  (bind _output_get (set `CharacterMovementComponent.MaxWalkSpeed` (select `/Game/Enemy/Enum/E_LocomotionState` InLocomotionState :`NewEnumerator1` 200.0 :`NewEnumerator2` 300.0 :`NewEnumerator3` 500.0 :!type "Float (single-precision)") (`self.CharacterMovement`)))
  (return _output_get))

(fn `UserConstructionScript`
  (`parent.UserConstructionScript`))